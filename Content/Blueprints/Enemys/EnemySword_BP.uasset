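; Enemy sword Blueprint that damages the player during an enemy attack.
; Its EnemyAttackTrace event runs a short Pawn object line trace from the Box component, opposite its forward vector, ignoring all EnemyParent_BP actors.
; Any hit applies a small fixed damage to player character 0, without checking which actor the trace struck.
; Nothing in this graph calls the event, and BeginPlay and Tick are empty.
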(event `self.ReceiveBeginPlay`)

(event `self.ReceiveTick`
  (params (DeltaSeconds :type "Float (single-precision)")))

(event `EnemyAttackTrace`
  (for _array_element (`|MakeArray` (`self.Box`))
    (bind _outactors (`GameplayStatics.GetAllActorsOfClass` "/Game/Blueprints/Enemys/EnemyParent_BP.EnemyParent_BP_C"))
    (bind _returnvalue (`SceneComponent.K2_GetComponentLocation` _array_element))
    (bind (_outhit _returnvalue_2) (`KismetSystemLibrary.LineTraceSingleForObjects` _returnvalue (- _returnvalue (* (`KismetMathLibrary.GetForwardVector` (`SceneComponent.K2_GetComponentRotation` _array_element)) 10.0)) (`|MakeArray` "ObjectTypeQuery3" :!type "EObjectTypeQuery Enum") true _outactors "None" true (struct :`R` 1.0 :`A` 1.0) (struct :`G` 1.0 :`A` 1.0) 0.2))
    (if _returnvalue_2
      (bind _asplayer_character (cast `/Game/Blueprints/Character/PlayerCharacter` (`GameplayStatics.GetPlayerCharacter` 0)))
      (`GameplayStatics.ApplyDamage` _asplayer_character 0.05))))

(fn `UserConstructionScript`)